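; BP_Bolts is a collectible container that scatters its bolts in an upward burst when play begins.
; On BeginPlay it loops over the direct children of its Scene component, reaching each Child Actor's root primitive.
; Each root gets a velocity-change impulse of random strength within an upward cone, so the launch ignores mass.
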(event `self.ReceiveBeginPlay`
  (for _array_element (`SceneComponent.GetChildrenComponents` (`self.Scene`) false)
    (bind _aschild_actor_component (cast `ChildActorComponent` _array_element))
    (bind _asprimitive_component (cast `PrimitiveComponent` (`Actor.RootComponent` (`ChildActorComponent.ChildActor` _aschild_actor_component))))
    (`PrimitiveComponent.AddImpulse` _asprimitive_component (* (`KismetMathLibrary.RandomUnitVectorInConeInDegrees` (0.0 0.0 1.0) 30.0) (`KismetMathLibrary.RandomFloatInRange` 400.0 900.0)) "None" true)))

(fn `UserConstructionScript`)